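; BP_Booktest03 is a test book prototype whose pages are turned by dragging left and right grab handles.
; While a handle is held, Tick maps its X offset from its anchor to PageProgress.
; Release snaps the handle back, flags Autopage and steps Page down (left) or up (right) past halfway.
; The Autopage animation and handle-visibility helpers are disconnected, and nothing here passes progress to the BP_BookPageTest child.
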(event `self.ReceiveBeginPlay`)

(event `/Game/_MAIN/_Common/BP/Interfaces/BPI_GrabHandleInteraction.OnGrab`
  (params (isLeftHandle :type Boolean))
  (if isLeftHandle
    (`self.SetGrabbed` "NewEnumerator1")
    (else
      (`self.SetGrabbed` "NewEnumerator2"))))

(event `/Game/_MAIN/_Common/BP/Interfaces/BPI_GrabHandleInteraction.OnRelease`
  (params (isLeftHandle :type Boolean))
  (bind _bp_grabhandle_r (`self.BP_GrabHandle_R`))
  (bind _bp_grabhandle_l (`self.BP_GrabHandle_L`))
  (bind _returnvalue (>= (`self.pageProgress`) 0.5))
  (bind _returnvalue_2 (>= (`self.pageProgress`) 0.5))
  (if isLeftHandle
    (set `self.pageGrabStatus` "NewEnumerator0")
    (`SceneComponent.K2_AttachToComponent` _bp_grabhandle_l (`self.SceneL`) "None" "KeepRelative" "KeepRelative" "KeepWorld" true)
    (`SceneComponent.K2_SetRelativeLocation` _bp_grabhandle_l (0.0 0.0 0.0) false false)
    (cast `/Game/_MAIN/_Common/BP/BP_BookPageTest` (`ChildActorComponent.ChildActor` (`self.BP_BookPageTest`)))
    (set `self.isGoForward` _returnvalue)
    (set `self.autopage` true)
    (if _returnvalue
      (`/Engine/EditorBlueprintResources/StandardMacros.DecrementInt` (`self.page`)))
    (else
      (set `self.pageGrabStatus` "NewEnumerator0")
      (`SceneComponent.K2_AttachToComponent` _bp_grabhandle_r (`self.SceneR`) "None" "KeepRelative" "KeepRelative" "KeepWorld" true)
      (`SceneComponent.K2_SetRelativeLocation` _bp_grabhandle_r (0.0 0.0 0.0) false false)
      (cast `/Game/_MAIN/_Common/BP/BP_BookPageTest` (`ChildActorComponent.ChildActor` (`self.BP_BookPageTest`)))
      (set `self.isGoForward` _returnvalue_2)
      (set `self.autopage` true)
      (if _returnvalue_2
        (`/Engine/EditorBlueprintResources/StandardMacros.IncrementInt` (`self.page`))))))

(event `self.ReceiveTick`
  (params (DeltaSeconds :type "Float (single-precision)"))
  (bind _pagegrabstatus (`self.pageGrabStatus`))
  (bind _returnvalue_x (`KismetMathLibrary.BreakVector` (- (`SceneComponent.K2_GetComponentLocation` (`self.BP_GrabHandle_R`)) (`SceneComponent.K2_GetComponentLocation` (`self.SceneR`)))))
  (bind _returnvalue_x_2 (`KismetMathLibrary.BreakVector` (- (`SceneComponent.K2_GetComponentLocation` (`Actor.RootComponent` (`ChildActorComponent.ChildActor` (`self.BP_GrabHandle_L`)))) (`SceneComponent.K2_GetComponentLocation` (`self.SceneL`)))))
  (if (`|EnumInequality` _pagegrabstatus "NewEnumerator0")
    (set `self.pageProgress` (select `/Game/_MAIN/_Common/BP/Enums/E_PageGrabStatus` _pagegrabstatus :`NewEnumerator1` (`KismetMathLibrary.MapRangeClamped` _returnvalue_x_2 0.0 240.0 1.0) :`NewEnumerator2` (`KismetMathLibrary.MapRangeClamped` _returnvalue_x 0.0 -240.0 0.0 1.0)))
    (set `self.distanceR` _returnvalue_x)
    (set `self.distanceL` _returnvalue_x_2)))

(fn `ResetHandles`
  (params (pageGrabStatus :type "/Game/_MAIN/_Common/BP/Enums/E_PageGrabStatus Enum" :default "NewEnumerator0") (Target :type "SceneComponent Object Reference") (Parent :type "SceneComponent Object Reference") (isNextPage :type Boolean))
  (bind _returnvalue (>= (`self.pageProgress`) 0.5))
  (set `self.pageGrabStatus` pageGrabStatus)
  (`SceneComponent.K2_AttachToComponent` Target Parent "None" "KeepRelative" "KeepRelative" "KeepWorld" true)
  (`SceneComponent.K2_SetRelativeLocation` Target (0.0 0.0 0.0) false false)
  (cast `/Game/_MAIN/_Common/BP/BP_BookPageTest` (`ChildActorComponent.ChildActor` (`self.BP_BookPageTest`)))
  (set `self.isGoForward` _returnvalue)
  (set `self.autopage` true)
  (`self.UpdatePage` _returnvalue (`local.isNextPage`)))

(fn `SetGrabbed`
  (params (pageGrabStatus :type "/Game/_MAIN/_Common/BP/Enums/E_PageGrabStatus Enum" :default "NewEnumerator0"))
  (set `self.pageGrabStatus` pageGrabStatus)
  (set `self.autopage` false))

(fn `SetPageHandleVisibility`
  (bind _asbp_book_page_test (cast `/Game/_MAIN/_Common/BP/BP_BookPageTest` (`ChildActorComponent.ChildActor` (`self.BP_BookPageTest`))))
  (`self.ToggleHandles` (not (>= (`self.page`) (`KismetArrayLibrary.Array_LastIndex` (`/Game/_MAIN/_Common/BP/BP_BookPageTest.pageMatList` _asbp_book_page_test)))) (`self.BP_GrabHandle_R`))
  (`self.ToggleHandles` (not (<= (`self.page`) 0)) (`self.BP_GrabHandle_L`)))

(fn `SetReleased`
  (params (pageGrabStatus :type "/Game/_MAIN/_Common/BP/Enums/E_PageGrabStatus Enum" :default "NewEnumerator0"))
  (switch `/Game/_MAIN/_Common/BP/Enums/E_PageGrabStatus` (`self.pageGrabStatus`)))

(fn `ToggleHandles`
  (params (doEnable :type Boolean) (handleComponentRef :type "ChildActorComponent Object Reference"))
  (`SceneComponent.SetVisibility` handleComponentRef doEnable true)
  (if doEnable
    (`ActorComponent.Activate` handleComponentRef false)
    (else
      (`ActorComponent.Deactivate` handleComponentRef))))

(fn `UpdatePage`
  (params (isOverThreshold :type Boolean) (isNextPage :type Boolean))
  (if isOverThreshold
    (bind _output_get (set `self.page` (+ (stale _output_get) (`KismetMathLibrary.SelectInt` 1 -1 isNextPage))))
    (`self.SetPageHandleVisibility`)))

(fn `UserConstructionScript`)