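; Prototype interactive book whose pages are turned by grabbing and dragging left and right handles.
; While a handle is held, Tick maps its X offset from its anchor to a normalized PageProgress.
; On release, the handle reattaches at its anchor, a 0.5 progress threshold decides the page index change, and handles hide at the child BP_BookPageTest's first and last page.
; The auto-page animation is deprecated and disconnected.
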(event `self.ReceiveBeginPlay`
  (`self.SetPageHandleVisibility`))

(event `self.GrabComponent_R.OnGrabbed`
  (`self.SetGrabbed` "NewEnumerator2"))

(event `self.GrabComponent_L.OnGrabbed`
  (`self.SetGrabbed` "NewEnumerator1"))

(event `self.GrabComponent_R.OnDropped`
  (`self.ResetHandles` "NewEnumerator0" (`self.GrabSphere_R`) (`self.SceneR`) true))

(event `self.GrabComponent_L.OnDropped`
  (`self.ResetHandles` "NewEnumerator0" (`self.GrabSphere_L`) (`self.SceneL`)))

(event `self.ReceiveTick`
  (params (DeltaSeconds :type "Float (single-precision)"))
  (bind _pagegrabstatus (`self.pageGrabStatus`))
  (bind _returnvalue_x (`KismetMathLibrary.BreakVector` (- (`SceneComponent.K2_GetComponentLocation` (`self.GrabSphere_R`)) (`SceneComponent.K2_GetComponentLocation` (`self.SceneR`)))))
  (bind _returnvalue_x_2 (`KismetMathLibrary.BreakVector` (- (`SceneComponent.K2_GetComponentLocation` (`self.GrabSphere_L`)) (`SceneComponent.K2_GetComponentLocation` (`self.SceneL`)))))
  (if (`|EnumInequality` _pagegrabstatus "NewEnumerator0")
    (set `self.pageProgress` (select `/Game/_MAIN/_Common/BP/Enums/E_PageGrabStatus` _pagegrabstatus :`NewEnumerator1` (`KismetMathLibrary.MapRangeClamped` _returnvalue_x_2 0.0 240.0 1.0) :`NewEnumerator2` (`KismetMathLibrary.MapRangeClamped` _returnvalue_x 0.0 -240.0 0.0 1.0)))))

(fn `ResetHandles`
  (params (pageGrabStatus :type "/Game/_MAIN/_Common/BP/Enums/E_PageGrabStatus Enum" :default "NewEnumerator0") (Target :type "SceneComponent Object Reference") (Parent :type "SceneComponent Object Reference") (isNextPage :type Boolean))
  (bind _returnvalue (>= (`self.pageProgress`) 0.5))
  (set `self.pageGrabStatus` pageGrabStatus)
  (`SceneComponent.K2_AttachToComponent` Target Parent "None" "KeepRelative" "KeepRelative" "KeepWorld" true)
  (`SceneComponent.K2_SetRelativeLocation` Target (0.0 0.0 0.0) false false)
  (cast `/Game/_MAIN/_Common/BP/BP_BookPageTest` (`ChildActorComponent.ChildActor` (`self.BP_BookPageTest`)))
  (set `self.isGoForward` _returnvalue)
  (set `self.autopage` true)
  (`self.UpdatePage` _returnvalue (`local.isNextPage`)))

(fn `SetGrabbed`
  (params (pageGrabStatus :type "/Game/_MAIN/_Common/BP/Enums/E_PageGrabStatus Enum" :default "NewEnumerator0"))
  (set `self.pageGrabStatus` pageGrabStatus)
  (set `self.autopage` false))

(fn `SetPageHandleVisibility`
  (bind _asbp_book_page_test (cast `/Game/_MAIN/_Common/BP/BP_BookPageTest` (`ChildActorComponent.ChildActor` (`self.BP_BookPageTest`))))
  (`self.ToggleHandles` (not (== (`self.page`) (`KismetArrayLibrary.Array_LastIndex` (`/Game/_MAIN/_Common/BP/BP_BookPageTest.pageMatList` _asbp_book_page_test)))) (`self.GrabSphere_R`))
  (`self.ToggleHandles` (not (== (`self.page`) 0)) (`self.GrabSphere_L`)))

(fn `SetReleased`
  (params (pageGrabStatus :type "/Game/_MAIN/_Common/BP/Enums/E_PageGrabStatus Enum" :default "NewEnumerator0"))
  (switch `/Game/_MAIN/_Common/BP/Enums/E_PageGrabStatus` (`self.pageGrabStatus`)))

(fn `ToggleHandles`
  (params (doEnable :type Boolean) (handleComponentRef :type "StaticMeshComponent Object Reference"))
  (`SceneComponent.SetVisibility` handleComponentRef doEnable true)
  (if doEnable
    (`ActorComponent.Activate` handleComponentRef false)
    (else
      (`ActorComponent.Deactivate` handleComponentRef))))

(fn `UpdatePage`
  (params (isOverThreshold :type Boolean) (isNextPage :type Boolean))
  (bind _page (`self.page`))
  (if isOverThreshold
    (if isNextPage
      (`/Engine/EditorBlueprintResources/StandardMacros.IncrementInt` _page
        (:`  `
          _))
      (else
        (`/Engine/EditorBlueprintResources/StandardMacros.DecrementInt` _page
          (:`  `
            _))))
    (`self.SetPageHandleVisibility`)))

(fn `UserConstructionScript`)