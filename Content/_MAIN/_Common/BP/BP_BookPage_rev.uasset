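; Book page actor that gives its PagLibro component a randomized look when spawned, marked as work in progress.
; On BeginPlay, material slots 0 and 1 each get an independent coin-flip pick between the first two PageMatList entries, so both can match.
; A DestroyPage event removes the actor; overlap, tick and construction logic are empty.
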(event `self.ReceiveBeginPlay`
  (bind _paglibro (`self.PagLibro`))
  (bind _output (`|GetArrayItem` (`self.pageMatList`) (`KismetMathLibrary.SelectInt` 0 1 (> (`KismetMathLibrary.RandomFloat`) 0.5))))
  ;[1 1 0] WIP
  (`PrimitiveComponent.SetMaterial` _paglibro 0 _output)
  (`PrimitiveComponent.SetMaterial` _paglibro 1 _output))

(event `DestroyPage`
  (`self.K2_DestroyActor`))

(fn `UserConstructionScript`)