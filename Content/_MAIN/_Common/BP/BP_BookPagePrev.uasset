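; BP_BookPagePrev is a book page actor, apparently for the previous page, that applies page visuals when given a page.
; Its SetPage event passes the page to SetPageMaterials, whose body is not defined here, then prints the parent actor's display name as debug output.
; BeginPlay and the construction script only call their parent versions, and Tick and overlap events are disabled.
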(event `self.ReceiveBeginPlay`
  (`parent.ReceiveBeginPlay`))

(event `/Game/_MAIN/_Common/BP/Interfaces/BPI_Page.SetPage`
  (params (page :type Integer))
  (`self.SetPageMaterials` page)
  (`KismetSystemLibrary.PrintString` (`KismetSystemLibrary.GetDisplayName` (`self.GetParentActor`))))

(fn `UserConstructionScript`
  (`parent.UserConstructionScript`))