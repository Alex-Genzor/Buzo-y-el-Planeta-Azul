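; Test Blueprint for an animated book page (PagLibro), apparently an unfinished prototype.
; BeginPlay sets the page animation to its start without firing notifies.
; VolverASuSitio ("return to its place") enables Autopagina and stores two incoming values, but the Tick branch on that flag does nothing yet.
; Disconnected leftover nodes set play rate, swap the animation and print its length.
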(event `self.ReceiveBeginPlay`
  (`SkeletalMeshComponent.SetPosition` (`self.PagLibro`) 0.0 false))

(event `VolverASuSitio`
  (params (NewParam :type Boolean) (NewParam2 :type "Float (double-precision)"))
  (set `self.Autopagina` true)
  (set `self.NewVar_0` NewParam)
  (set `self.position` NewParam2))

(event `self.ReceiveTick`
  (params (DeltaSeconds :type "Float (single-precision)"))
  (if (`self.Autopagina`)
    _))

(fn `UserConstructionScript`)