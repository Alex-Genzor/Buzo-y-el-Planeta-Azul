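; BP_Booktest04 is a test book actor with grabbable page handles and a BP_BookPageTest child actor for the page.
; Grabbing records the grab status and stops auto-paging; ResetHandles re-attaches a handle, resumes auto-paging and changes the page if progress reaches halfway.
; Handle visibility and activation follow the page index against the child's material list bounds.
; Prev/Next button handling and the SetReleased switch are largely unfinished.
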(event `self.ReceiveBeginPlay`)

(event `/Game/_MAIN/_Common/BP/Interfaces/BPI_ButtonInteraction.ButtonInteraction`
  (params (buttonID :type String))
  (bind _page (`self.page`))
  (switch `string` buttonID
    (:`prev`
      (if (<= _page 0)
        _))
    (:`next`
      (`/Engine/EditorBlueprintResources/StandardMacros.IncrementInt` _page
        (:`  `
          (cast `/Game/_MAIN/_Common/BP/BP_BookPageTest` (`ChildActorComponent.ChildActor` (`self.BP_BookPageTest`))))))))

(fn `ResetHandles`
  (params (pageGrabStatus :type "/Game/_MAIN/_Common/BP/Enums/E_PageGrabStatus Enum" :default "NewEnumerator0") (Target :type "SceneComponent Object Reference") (Parent :type "SceneComponent Object Reference") (isNextPage :type Boolean))
  (bind _returnvalue (>= (`self.pageProgress`) 0.5))
  (set `self.pageGrabStatus` pageGrabStatus)
  (`SceneComponent.K2_AttachToComponent` Target Parent "None" "KeepRelative" "KeepRelative" "KeepWorld" true)
  (`SceneComponent.K2_SetRelativeLocation` Target (0.0 0.0 0.0) false false)
  (cast `/Game/_MAIN/_Common/BP/BP_BookPageTest` (`ChildActorComponent.ChildActor` (`self.BP_BookPageTest`)))
  (set `self.isGoForward` _returnvalue)
  (set `self.autopage` true)
  (`self.UpdatePage` _returnvalue (`local.isNextPage`)))

(fn `SetGrabbed`
  (params (pageGrabStatus :type "/Game/_MAIN/_Common/BP/Enums/E_PageGrabStatus Enum" :default "NewEnumerator0"))
  (set `self.pageGrabStatus` pageGrabStatus)
  (set `self.autopage` false))

(fn `SetPageHandleVisibility`
  (bind _asbp_book_page_test (cast `/Game/_MAIN/_Common/BP/BP_BookPageTest` (`ChildActorComponent.ChildActor` (`self.BP_BookPageTest`))))
  (`self.ToggleHandles` (not (>= (`self.page`) (`KismetArrayLibrary.Array_LastIndex` (`/Game/_MAIN/_Common/BP/BP_BookPageTest.pageMatList` _asbp_book_page_test)))) null)
  (`self.ToggleHandles` (not (<= (`self.page`) 0)) null))

(fn `SetReleased`
  (params (pageGrabStatus :type "/Game/_MAIN/_Common/BP/Enums/E_PageGrabStatus Enum" :default "NewEnumerator0"))
  (switch `/Game/_MAIN/_Common/BP/Enums/E_PageGrabStatus` (`self.pageGrabStatus`)))

(fn `ToggleHandles`
  (params (doEnable :type Boolean) (handleComponentRef :type "ChildActorComponent Object Reference"))
  (`SceneComponent.SetVisibility` handleComponentRef doEnable true)
  (if doEnable
    (`ActorComponent.Activate` handleComponentRef false)
    (else
      (`ActorComponent.Deactivate` handleComponentRef))))

(fn `UpdatePage`
  (params (isOverThreshold :type Boolean) (isNextPage :type Boolean))
  (if isOverThreshold
    (bind _output_get (set `self.page` (+ (stale _output_get) (`KismetMathLibrary.SelectInt` 1 -1 isNextPage))))
    (`self.SetPageHandleVisibility`)))

(fn `UserConstructionScript`)