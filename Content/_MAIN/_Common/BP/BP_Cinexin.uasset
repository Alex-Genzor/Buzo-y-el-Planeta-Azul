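; BP_Cinexin is a grabbable, crank-style control that turns a pivot to follow a handle sphere.
; While grabbed, Tick takes the direction from RotRef to Sphere, sets RotRef's world rotation from only the clamped quaternion Y component, and stores it in NewVar.
; GrabComponent events toggle the grabbed state, and dropping reattaches Sphere to Snap at zero offset.
; An interpolated look-at version and a debug print remain unconnected.
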(event `self.ReceiveTick`
  (params (DeltaSeconds :type "Float (single-precision)"))
  (bind (_returnvalue_x _returnvalue_y) (`KismetMathLibrary.BreakQuat` (`KismetMathLibrary.Conv_RotatorToQuaternion` (`KismetMathLibrary.Conv_VectorToRotator` (`KismetMathLibrary.GetDirectionUnitVector` (`SceneComponent.K2_GetComponentLocation` (`self.RotRef`)) (`SceneComponent.K2_GetComponentLocation` (`self.Sphere`)))))))
  (bind _returnvalue (`KismetMathLibrary.Quat_Rotator` (`KismetMathLibrary.MakeQuat` 0.0 (`KismetMathLibrary.ClampAxis` _returnvalue_y))))
  (if (`self.isGrabbed`)
    (`SceneComponent.K2_SetWorldRotation` (`self.RotRef`) _returnvalue false false)
    (set `self.NewVar` _returnvalue)))

(event `self.GrabComponent.OnDropped`
  (bind _sphere (`self.Sphere`))
  (`SceneComponent.K2_AttachToComponent` _sphere (`self.Snap`) "None" "KeepRelative" "KeepRelative" "KeepRelative" true)
  (`SceneComponent.K2_SetRelativeLocation` _sphere (0.0 0.0 0.0) false false)
  (set `self.isGrabbed` false))

(event `self.GrabComponent.OnGrabbed`
  (set `self.isGrabbed` true))

(fn `UserConstructionScript`)