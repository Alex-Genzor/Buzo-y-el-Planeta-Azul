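; BP_Cinexin3 is an interactive Cinexin prop whose animation and screen image toggle on a button interaction.
; BeginPlay creates a dynamic instance of MI_Pantalla and assigns it to the Cinexin mesh's second material slot.
; ButtonInteraction flips PlayAnim, which drives both the mesh's global animation rate and the material's ToggleImage parameter, so motion and image switch together.
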(event `self.ReceiveBeginPlay`
  (bind _returnvalue (`KismetMaterialLibrary.CreateDynamicMaterialInstance` "/Game/_MAIN/_Common/Materials/MI_Pantalla.MI_Pantalla"))
  (bind _output_get (set `self.material` _returnvalue))
  (`PrimitiveComponent.SetMaterial` (`self.cinexin`) 1 _output_get))

(event `self.ReceiveTick`
  (params (DeltaSeconds :type "Float (single-precision)")))

(event `self.ButtonInteraction`
  (params (buttonID :type String))
  (bind _output_get (set `self.playAnim` (not (stale _output_get))))
  (bind _returnvalue (`KismetMathLibrary.SelectFloat` 1.0 0.0 _output_get))
  (set `SkeletalMeshComponent.GlobalAnimRateScale` _returnvalue (`self.cinexin`))
  (`MaterialInstanceDynamic.SetScalarParameterValue` (`self.material`) "ToggleImage" _returnvalue))

(fn `UserConstructionScript`)