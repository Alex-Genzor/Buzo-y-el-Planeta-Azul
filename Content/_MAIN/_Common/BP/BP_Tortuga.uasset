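; Turtle actor that has trash pieces removed from it, one per touch by a hand collider.
; When its Box begins an overlap, GetHands parses the component's display name to check for a "HandCollider" prefix before the underscore.
; Each matching overlap increments TrashCounter, with the first two destroying BasuraN0 and then BasuraN1.
; GetHands also derives left or right hand from the name suffix, but that result is unused.
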(event `self.ReceiveBeginPlay`)

(event `self.Box.OnComponentBeginOverlap`
  (params (OverlappedComponent :type "PrimitiveComponent Object Reference") (OtherActor :type "Actor Object Reference") (OtherComp :type "PrimitiveComponent Object Reference") (OtherBodyIndex :type Integer) (bFromSweep :type Boolean) (SweepResult :type "HitResult Structure (by ref)"))
  (bind _iswantedcollider (`self.GetHands` null null "HandCollider" "_"))
  (if _iswantedcollider
    (switch `int` (`self.trashCounter`)
      (:`0`
        (`ActorComponent.K2_DestroyComponent` (`self.BasuraN0`)))
      (:`1`
        (`ActorComponent.K2_DestroyComponent` (`self.BasuraN1`))))
    (bind _output_get (set `self.trashCounter` (+ (stale _output_get) 1)))))

(fn `GetHands`
  (params (otherActor :type "Actor Object Reference") (otherComp :type "PrimitiveComponent Object Reference") (colliderName :type String) (separatorChar :type String))
  (returns (isWantedCollider :type Boolean) (isLeftHand :type Boolean))
  (bind (_lefts _rights) (`KismetStringLibrary.Split` (`KismetStringLibrary.Replace` (`KismetSystemLibrary.GetDisplayName` otherComp) (`KismetStringLibrary.Concat_StrStr` (`KismetSystemLibrary.GetDisplayName` otherActor) ".")) separatorChar))
  (return (== _lefts colliderName) (== _rights "L")))

(fn `UserConstructionScript`)