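; Deprecated VR interactable actor that toggles a PlayAnim flag when an overlapping hand pulls its trigger.
; Cube overlap identifies left or right HandCollider by parsing component display names, then enables input and adds an Enhanced Input mapping context.
; Any end overlap clears the hand state, disables input and removes the context.
; PlayAnim is only printed every Tick here; ButtonInteraction is an empty stub.
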(event `self.ReceiveTick`
  (params (DeltaSeconds :type "Float (single-precision)"))
  (`KismetSystemLibrary.PrintString` (`KismetStringLibrary.Conv_BoolToString` (`self.playAnim`))))

(event `self.Cube.OnComponentBeginOverlap`
  (params (OverlappedComponent :type "PrimitiveComponent Object Reference") (OtherActor :type "Actor Object Reference") (OtherComp :type "PrimitiveComponent Object Reference") (OtherBodyIndex :type Integer) (bFromSweep :type Boolean) (SweepResult :type "HitResult Structure (by ref)"))
  (bind _returnvalue (`GameplayStatics.GetPlayerController` 0))
  (bind (_lefts _rights) (`KismetStringLibrary.Split` (`KismetStringLibrary.Replace` (`KismetSystemLibrary.GetDisplayName` OtherComp) (`KismetStringLibrary.Concat_StrStr` (`KismetSystemLibrary.GetDisplayName` OtherActor) ".")) "_"))
  (if (== _lefts "HandCollider")
    (set `self.handOverlap` (select `bool` (== _rights "L") :`false` "NewEnumerator2" :`true` "NewEnumerator1" :!type "/Game/_MAIN/_Common/BP/Enums/E_HandOverlap Enum"))
    (`self.EnableInput` _returnvalue)
    (`EnhancedInputSubsystemInterface.AddMappingContext` (pcsubsystem `EnhancedInputLocalPlayerSubsystem` _returnvalue) (`self.mapContext`) 1 (struct))))

(event `self.Cube.OnComponentEndOverlap`
  (params (OverlappedComponent :type "PrimitiveComponent Object Reference") (OtherActor :type "Actor Object Reference") (OtherComp :type "PrimitiveComponent Object Reference") (OtherBodyIndex :type Integer))
  (bind _returnvalue (`GameplayStatics.GetPlayerController` 0))
  (set `self.handOverlap` "NewEnumerator0")
  (`self.DisableInput` _returnvalue)
  (`EnhancedInputSubsystemInterface.RemoveMappingContext` (pcsubsystem `EnhancedInputLocalPlayerSubsystem` _returnvalue) (`self.mapContext`) (struct)))

(event `EnhancedInput|/Game/_MAIN/_Alex/Input/InteractionSystemA/IA_VrTriggerL`
  (params (ActionValue :type "Float (double-precision)") (ElapsedSeconds :type "Float (double-precision)") (TriggeredSeconds :type "Float (double-precision)") (InputAction :type "InputAction Object Reference" :default "/Game/_MAIN/_Alex/Input/InteractionSystemA/IA_VrTriggerL.IA_VrTriggerL"))
  (:`Started`
    (if (`|EnumEquality` (`self.handOverlap`) "NewEnumerator1")
      (bind _output_get (set `self.playAnim` (not (stale _output_get)) :!label _label)))))

(event `EnhancedInput|/Game/_MAIN/_Alex/Input/InteractionSystemA/IA_VrTriggerR`
  (params (ActionValue :type "Float (double-precision)") (ElapsedSeconds :type "Float (double-precision)") (TriggeredSeconds :type "Float (double-precision)") (InputAction :type "InputAction Object Reference" :default "/Game/_MAIN/_Alex/Input/InteractionSystemA/IA_VrTriggerR.IA_VrTriggerR"))
  (:`Started`
    (if (`|EnumEquality` (`self.handOverlap`) "NewEnumerator2")
      (goto _label))))

(event `/Game/_MAIN/_Common/BP/Interfaces/BPI_ButtonInteraction.ButtonInteraction`
  (params (buttonID :type String)))

(fn `UserConstructionScript`)