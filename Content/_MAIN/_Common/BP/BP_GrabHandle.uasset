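; BP_GrabHandle is a grabbable handle actor that reports grab and release to its parent actor, identifying itself as the left handle or not.
; Its GrabComponent events send OnGrabMessage or OnReleaseMessage to the parent with the IsLeftHandle flag and toggle a Grab boolean.
; While Grab is true, Tick prints the handle's world location as debug output.
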(event `self.ReceiveTick`
  (params (DeltaSeconds :type "Float (single-precision)"))
  (if (`self.grab`)
    (`KismetSystemLibrary.PrintString` (`KismetStringLibrary.Conv_VectorToString` (`self.K2_GetActorLocation`)))))

(event `self.GrabComponent.OnGrabbed`
  (message `/Game/_MAIN/_Common/BP/Interfaces/BPI_GrabHandleInteraction.OnGrab` (`self.GetParentActor`) (`self.isLeftHandle`))
  (set `self.grab` true))

(event `self.GrabComponent.OnDropped`
  (message `/Game/_MAIN/_Common/BP/Interfaces/BPI_GrabHandleInteraction.OnRelease` (`self.GetParentActor`) (`self.isLeftHandle`))
  (set `self.grab` false))

(fn `UserConstructionScript`)